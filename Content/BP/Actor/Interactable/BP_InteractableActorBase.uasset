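; Base actor for interactable items that go into a grid-based inventory, with an empty HasInteracted event.
; PopupRootInventory creates a new UI_RootInventory, stores it on BP_FPSCon, shows it, and spawns this item into the grid, keeping the result as GridSlot.
; RotateItem swaps the item's grid and image dimensions on every call, returning the new size and a quarter-turn or zero angle chosen by IsA.
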(event `/Game/BP/Interface/BPI_Interact.HasInteracted`)

(fn `PopupRootInventory`
  (bind _returnvalue (`|CreateWidget` "/Game/BP/UI/DnDUI/UI_RootInventory.UI_RootInventory_C"))
  (bind _output_get (set `/Game/BP/BP_FPSCon.UI_RootInventory` _returnvalue (cast `/Game/BP/BP_FPSCon` (`GameplayStatics.GetPlayerController` 0) :!pure true)))
  (`UserWidget.AddToViewport` _output_get 0)
  (bind _gridslot (`/Game/BP/UI/DnDUI/UI_RootInventory.SpawnItemToGrid` _returnvalue (`self.ItemXSize`) (`self.ItemYSize`) (`self.ItemSize`) (`self.ItemImage`) self))
  (set `self.GridSlot` _gridslot))

(fn `RotateItem`
  (params (isA :type Boolean))
  (returns (ItemSize :type "Vector2D Structure") (Angle :type "Float (double-precision)"))
  (locals (vr_value :type Integer))
  (bind (_itemsize_x _itemsize_y) (`KismetMathLibrary.BreakVector2D` (`self.ItemSize`)))
  (set `self.Angle` (`KismetMathLibrary.SelectFloat` 0.25 0.0 isA))
  (set `local.vr_value` (`self.ItemXSize`))
  (set `self.ItemXSize` (`self.ItemYSize`))
  (set `self.ItemYSize` (`local.vr_value`))
  (bind _output_get (set `self.ItemSize` (`KismetMathLibrary.MakeVector2D` _itemsize_y _itemsize_x)))
  (return _output_get (`self.Angle`)))

(fn `UserConstructionScript`)