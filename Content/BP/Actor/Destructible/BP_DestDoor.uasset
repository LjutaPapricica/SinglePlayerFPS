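; BP_DestDoor is a destructible door that swings open or closed on interaction and breaks apart under damage.
; HasInteracted uses a FlipFlop to play or reverse a rotation timeline.
; Destroy applies radial damage at the hit point and drains clamped door HP.
; At zero HP, it fires damage bursts once at preset destroy points to shatter the mesh, then removes the door after a delay.
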(event `self.ReceiveBeginPlay`
  (`ActorComponent.K2_DestroyComponent` (`self.BoxTrigger`)))

(event `/Game/BP/Interface/BPI_Destruction.Destroy`
  (params (Damage :type "Float (single-precision)") (HitPos :type "Vector Structure"))
  ;[1 1 1] Comment
  (`DestructibleComponent.ApplyRadiusDamage` (`self.Door`) Damage HitPos 1.0 100.0 true)
  (bind _output_get (set `self.DoorHP` (`KismetMathLibrary.FClamp` (- (`self.DoorHP`) Damage) 0.0 1200.0)))
  (if (== _output_get 0.0)
    (`/Engine/EditorBlueprintResources/StandardMacros.DoOnce` false
      (:`Completed`
        (for _index (range 6)
          (`DestructibleComponent.ApplyRadiusDamage` (`self.Door`) 500.0 (`SceneComponent.K2_GetComponentLocation` (`|GetArrayItem` (`|MakeArray` (`self.DestroyPoint02`) (`self.DestroyPoint03`) (`self.DestroyPoint04`) (`self.DestroyPoint05`) (`self.DestroyPoint06`) (`self.DestroyPoint01`)) _index)) 100.0 1.0 true))
        (`KismetSystemLibrary.Delay` 3.0)
        (`KismetSystemLibrary.PrintString` "Destroyed" true true (struct :`R` 1.0 :`B` 0.018187 :`A` 1.0))
        (`ActorComponent.K2_DestroyComponent` (`self.Door`))))))

(event `/Game/BP/Interface/BPI_Interact.HasInteracted`
  (bind _doorrotanimation (`self.DoorRotAnimation`))
  (`/Engine/EditorBlueprintResources/StandardMacros.FlipFlop`
    (:`A`
      (`TimelineComponent.PlayFromStart` _doorrotanimation))
    (:`B`
      (`TimelineComponent.ReverseFromEnd` _doorrotanimation))))

(fn `UserConstructionScript`
  (`parent.UserConstructionScript`))