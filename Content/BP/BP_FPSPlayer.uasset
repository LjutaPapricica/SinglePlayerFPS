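; First-person player character that spawns and equips a BP_KAU weapon and handles movement, aiming, firing, reloading and item interaction.
; Firing emits noise, plays timeline recoil and feeds weapon spread, which grows per shot and decays on Tick.
; Reload and interact steer control rotation toward the weapon or left hand, with montages and IK messages to the AnimInstance.
; Traces position the crosshair and interact-bar widgets over world points.
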(event `self.ReceiveBeginPlay`
  ;[1 1 1] begin play
  (`|ExecutionSequence`
    (:`then_0`
      (bind _returnvalue (`|SpawnActorFromClass` "/Game/BP/Weapon/WeaponClass/BP_KAU.BP_KAU_C" (`KismetMathLibrary.MakeTransform` (0.0 0.0 0.0)) "AlwaysSpawn" "OverrideRootScale" null null))
      (bind _output_get (set `self.EquippingWeapon` _returnvalue))
      (`/Game/BP/Weapon/WeaponClass/BP_Gun.SpawnEquip` _output_get (`self.Mesh`)))
    (:`then_1`
      (message `/Game/BP/Interface/BPI_Animation.DecideHandIkEffector` (`SkeletalMeshComponent.GetAnimInstance` (`self.Mesh`)) (`.WeaponName_15_0E9F124B497C9B0E465B2198313C0803` (break `/Game/BP/Weapon/s_WeaponState` (`/Game/BP/Weapon/WeaponClass/BP_Gun.s_WeaponState` (`self.EquippingWeapon`))))))
    (:`then_2`
      (bind _returnvalue_2 (`|CreateWidget` "/Game/BP/UI/UI_Crosshair.UI_Crosshair_C"))
      (bind _output_get_2 (set `self.UI_Crosshair` _returnvalue_2))
      (`UserWidget.AddToViewport` _output_get_2 0)
      (bind _returnvalue_3 (`|CreateWidget` "/Game/BP/UI/UI_InteractBar.UI_InteractBar_C"))
      (set `self.UI_CircularBar` _returnvalue_3))
    (:`then_3`
      (`KismetSystemLibrary.K2_SetTimerDelegate` (`|CreateDelegate` :!event `PopUpInteractUI`) 0.01 true))))

(event `Recoil`
  ;[1 0 0] Custom Event
  (bind (_direction _alpha) (`Timeline|RecoilAnimation` :!via `PlayFromStart`)
    (:`Update`
      (`self.AddControllerPitchInput` (`KismetMathLibrary.Lerp` 0.0 -0.075 _alpha))
      (`self.AddControllerYawInput` (`KismetMathLibrary.Lerp` 0.0 (`KismetMathLibrary.RandomFloatInRange` (`KismetMathLibrary.RandomFloatInRange` -0.08 -0.045) (`KismetMathLibrary.RandomFloatInRange` 0.045 0.08)) _alpha)))))

(event `PopUpInteractUI`
  (bind _returnvalue (`GameplayStatics.GetPlayerCameraManager` 0))
  (bind _returnvalue_2 (`self.K2_GetActorLocation` _returnvalue))
  ;[1 0 0] Custom Event
  (bind (_outhit _returnvalue_3) (`KismetSystemLibrary.SphereTraceSingle` _returnvalue_2 (+ _returnvalue_2 (* (`KismetMathLibrary.GetForwardVector` (`self.K2_GetActorRotation` _returnvalue)) 250.0)) 20.0 "TraceTypeQuery1"))
  (bind (_bblockinghit _binitialoverlap _time _distance _location _impactpoint _normal _impactnormal _physmat _hitactor) (`GameplayStatics.BreakHitResult` _outhit))
  (if (and (`KismetSystemLibrary.IsValid` _hitactor) (`KismetSystemLibrary.DoesImplementInterface` _hitactor "/Game/BP/Interface/BPI_Interact.BPI_Interact_C"))
    (`|ExecutionSequence`
      (:`then_0`
        (`/Engine/EditorBlueprintResources/StandardMacros.DoOnce` false :!label _label
          (:`Completed`
            (`UserWidget.AddToViewport` (`self.UI_CircularBar`) 0))))
      (:`then_1`
        (`/Game/BP/UI/UI_InteractBar.SetBarToWorld` (`self.UI_CircularBar`) _returnvalue_3 (`SceneComponent.K2_GetComponentLocation` (`/Game/BP/Actor/Interactable/BP_InteractableActorBase.GazePoint` (cast `/Game/BP/Actor/Interactable/BP_InteractableActorBase` _hitactor :!pure true))))))
    (else
      (`Widget.RemoveFromParent` (`self.UI_CircularBar`))
      (goto _label :!via `Reset`))))

(event `CancelInteract`
  (bind _itemsearchsphere (`self.ItemSearchSphere`))
  ;[1 0 0] Custom Event
  (`AnimInstance.Montage_Resume` (`self.GetAnimInst`) "/Game/AnimStarterPack/InteractMontage.InteractMontage")
  (`/Engine/EditorBlueprintResources/StandardMacros.IsValid` _itemsearchsphere
    (:`Is Valid`
      (`ActorComponent.K2_DestroyComponent` _itemsearchsphere))))

(event `self.ReceiveTick`
  (params (DeltaSeconds :type "Float (single-precision)"))
  (bind _returnvalue (`SceneComponent.GetSocketLocation` (`/Game/BP/Weapon/WeaponClass/BP_Gun.GunMesh` (`self.EquippingWeapon`)) "MuzzleFlashSocket"))
  ;[1 1 1] Tick
  (`|ExecutionSequence`
    (:`then_0`
      (`self.TimeElapsedDecreaseSpread`))
    (:`then_1`
      (bind (_outhit _returnvalue_2) (`KismetSystemLibrary.LineTraceSingle` _returnvalue (+ _returnvalue (* (`KismetMathLibrary.GetForwardVector` (`self.K2_GetActorRotation` (`GameplayStatics.GetPlayerCameraManager` 0))) 20000.0)) "TraceTypeQuery1"))
      (`/Game/BP/UI/UI_Crosshair.SetHUDToWorld` (`self.UI_Crosshair`) _returnvalue_2 (`.ImpactPoint` (`GameplayStatics.BreakHitResult` _outhit))))))

(fn `CalculateLoudness`
  (returns (Loudness :type "Float (double-precision)"))
  (return (`KismetMathLibrary.MapRangeClamped` (`KismetMathLibrary.VSize` (`self.GetVelocity`)) 0.0 450.0 0.0 1.0)))

(fn `DecreaseSpread`
  (params (`Decrease Amount` :type "Float (double-precision)"))
  (bind _returnvalue (- (`self.SpreadCurrent`) `Decrease Amount`))
  (if (<= _returnvalue (`self.SpreadMin`))
    (set `self.SpreadCurrent` (`self.SpreadMin`))
    (else
      (set `self.SpreadCurrent` _returnvalue))))

(fn `EndAim`
  (`UserWidget.AddToViewport` (`self.UI_Crosshair`) 0)
  (`/Game/BP/Weapon/WeaponClass/BP_Gun.EndAim` (`self.EquippingWeapon`) self))

(fn `Fire`
  (bind _equippingweapon (`self.EquippingWeapon`))
  (bind _equippingweapon_2 (`self.EquippingWeapon`))
  (bind (_s_weaponstate_canselectfiringtype _s_weaponstate_pistol_ _s_weaponstate_clipsize _s_weaponstate_numofcanpenetrate _s_weaponstate_firerate _s_weaponstate_maxbulletspread _s_weaponstate_firespreadamount _s_weaponstate_fireingtype) (break `/Game/BP/Weapon/s_WeaponState` (`/Game/BP/Weapon/WeaponClass/BP_Gun.s_WeaponState` (`self.EquippingWeapon`))))
  (bind (_s_weaponstate_canselectfiringtype_2 _s_weaponstate_pistol__2 _s_weaponstate_clipsize_2 _s_weaponstate_numofcanpenetrate_2 _s_weaponstate_firerate_2 _s_weaponstate_maxbulletspread_2 _s_weaponstate_firespreadamount_2) (break `/Game/BP/Weapon/s_WeaponState` (`/Game/BP/Weapon/WeaponClass/BP_Gun.s_WeaponState` _equippingweapon)))
  (`PawnNoiseEmitterComponent.MakeNoise` (`self.PawnNoiseEmitter`) self 0.0 (`self.K2_GetActorLocation`))
  (`self.Recoil`)
  (if (`self.isAiming`)
    (message `/Game/BP/Weapon/BPI_Weapon.SendSpreadAmount` _equippingweapon 0.0)
    (else
      (message `/Game/BP/Weapon/BPI_Weapon.SendSpreadAmount` _equippingweapon (`self.SpreadCurrent`))))
  (`self.IncreaseSpread` _s_weaponstate_firespreadamount_2)
  (switch `/Game/BP/Weapon/e_WeaponFiringType` _s_weaponstate_fireingtype
    (:`NewEnumerator0`
      (`/Game/BP/Weapon/WeaponClass/BP_Gun.Fire` _equippingweapon_2))
    (:`NewEnumerator1`
      (`/Game/BP/Weapon/WeaponClass/BP_Gun.Fire` _equippingweapon_2)
      (bind _returnvalue (`KismetSystemLibrary.K2_SetTimerDelegate` (`|CreateDelegate` :!event `Fire`) (/ 1.0 _s_weaponstate_firerate) true))
      (set `self.FireHandle` _returnvalue))))

(fn `GazeToItem`
  (bind _returnvalue (`GameplayStatics.GetPlayerCameraManager` 0))
  (if (> (`self.InteractMontageLength`) 0.0)
    (`Controller.SetControlRotation` (`GameplayStatics.GetPlayerController` 0) (`KismetMathLibrary.RInterpTo` (`self.K2_GetActorRotation` _returnvalue) (`KismetMathLibrary.FindLookAtRotation` (`self.K2_GetActorLocation` _returnvalue) (`SceneComponent.GetSocketLocation` (`self.Mesh`) "hand_l")) (`GameplayStatics.GetWorldDeltaSeconds`) 2.0))
    (set `self.InteractMontageLength` (- (`self.InteractMontageLength`) (`GameplayStatics.GetWorldDeltaSeconds`)))
    (else
      (`KismetSystemLibrary.K2_PauseTimerHandle` (`self.InteractHandle`))
      (message `/Game/BP/Interface/BPI_Animation.EndInteract` (`self.GetAnimInst`)))))

(fn `GazeToPrevCameraRot`
  (set `self.isReloading` false)
  (if (> (`/Game/BP/Weapon/WeaponClass/BP_Gun.ReloadMontageLength` (`self.EquippingWeapon`)) 1.8)
    (`Controller.SetControlRotation` (`GameplayStatics.GetPlayerController` 0) (`KismetMathLibrary.RInterpTo` (`self.K2_GetActorRotation` (`GameplayStatics.GetPlayerCameraManager` 0)) (`self.PreCameraRot`) (`GameplayStatics.GetWorldDeltaSeconds`) 4.0))
    (`/Game/BP/Weapon/WeaponClass/BP_Gun.DecreaseMontageLength` (`self.EquippingWeapon`))
    (else
      (`self.FinishedSetControlRot`))))

(fn `GazeToWeapon`
  (bind _returnvalue (`GameplayStatics.GetPlayerCameraManager` 0))
  (set `self.isReloading` true)
  (`Controller.SetControlRotation` (`GameplayStatics.GetPlayerController` 0) (`KismetMathLibrary.RInterpTo` (`self.K2_GetActorRotation` _returnvalue) (`KismetMathLibrary.FindLookAtRotation` (`self.K2_GetActorLocation` _returnvalue) (`SceneComponent.K2_GetComponentLocation` (`/Game/BP/Weapon/WeaponClass/BP_Gun.GazePoint` (`self.EquippingWeapon`)))) (`GameplayStatics.GetWorldDeltaSeconds`) 8.0)))

(fn `IncreaseSpread`
  (params (`Increase Spread` :type "Float (double-precision)"))
  (bind _returnvalue (+ `Increase Spread` (`self.SpreadCurrent`)))
  (if (and (>= _returnvalue (`self.SpreadMax`)) (not (`self.isAiming`)))
    (set `self.SpreadCurrent` (`self.SpreadMax`))
    (else
      (set `self.SpreadCurrent` _returnvalue))))

(fn `Interact`
  (bind _itemsearchsphere (`self.ItemSearchSphere`))
  (bind _output (`|GetArrayItem` (`PrimitiveComponent.GetOverlappingActors` (`self.ItemSearchSphere`) "/Game/BP/Actor/Interactable/BP_InteractableActorBase.BP_InteractableActorBase_C")))
  (bind _returnvalue (`AddComponent|NODE_AddSphereComponent-0` :`bManualAttachment` true :`RelativeTransform` (`self.GetTransform`)))
  (bind _output_get (set `self.ItemSearchSphere` _returnvalue))
  (`PrimitiveComponent.SetCollisionEnabled` _output_get "QueryAndPhysics")
  (`SphereComponent.SetSphereRadius` _itemsearchsphere 120.0 true)
  (`PrimitiveComponent.SetCollisionResponseToChannel` _itemsearchsphere "ECC_GameTraceChannel1" "ECR_Ignore")
  (set `self.InteractedActor` _output)
  (if (and (`KismetSystemLibrary.IsValid` _output) (`KismetSystemLibrary.DoesImplementInterface` _output "/Game/BP/Interface/BPI_Interact.BPI_Interact_C"))
    (bind _returnvalue_2 (`AnimInstance.Montage_Play` (`self.GetAnimInst`) "/Game/AnimStarterPack/InteractMontage.InteractMontage" 1.0 "Duration" 0.0 false))
    (set `self.InteractMontageLength` _returnvalue_2)
    (message `/Game/BP/Interface/BPI_Animation.StartInteract` (`self.GetAnimInst`) (`SceneComponent.K2_GetComponentToWorld` (`/Game/BP/Actor/Interactable/BP_InteractableActorBase.GazePoint` (cast `/Game/BP/Actor/Interactable/BP_InteractableActorBase` (`self.InteractedActor`) :!pure true))))
    (bind _returnvalue_3 (`KismetSystemLibrary.K2_SetTimerDelegate` (`|CreateDelegate` :!event `GazeToItem`) (`GameplayStatics.GetWorldDeltaSeconds`) true))
    (set `self.InteractHandle` _returnvalue_3)))

(fn `InteractToItem`
  (bind _interactedactor (`self.InteractedActor`))
  (`/Engine/EditorBlueprintResources/StandardMacros.IsValid` _interactedactor
    (:`Is Valid`
      (message `/Game/BP/Interface/BPI_Interact.HasInteracted` _interactedactor)
      (`AnimInstance.Montage_Resume` (`self.GetAnimInst`) "/Game/AnimStarterPack/InteractMontage.InteractMontage"))
    (:`Is Not Valid`
      _))
  (return))

(fn `MovePlayer`
  (params (MoveDirection :type "Vector Structure") (MoveValue :type "Float (double-precision)"))
  (`self.AddMovementInput` MoveDirection MoveValue))

(fn `Reload`
  (set `self.PreCameraRot` (`self.GetControlRotation`))
  (`/Game/BP/Weapon/WeaponClass/BP_Gun.Reload` (`self.EquippingWeapon`)))

(fn `Run`
  (params (Alpha :type "Float (double-precision)"))
  (set `CharacterMovementComponent.MaxWalkSpeed` (`KismetMathLibrary.Lerp` 200.0 (`self.MaxWalkSpeed`) Alpha) (`self.CharacterMovement`)))

(fn `StartAim`
  (`Widget.RemoveFromParent` (`self.UI_Crosshair`))
  (`/Game/BP/Weapon/WeaponClass/BP_Gun.StartAim` (`self.EquippingWeapon`))
  (`self.FinishedSetControlRot`))

(fn `TimeElapsedDecreaseSpread`
  (if (>= (`self.SpreadCurrent`) (`self.SpreadMin`))
    (`self.DecreaseSpread` (* (`self.SpreadDecreaseSpeed`) (`GameplayStatics.GetWorldDeltaSeconds`)))))

(fn `UserConstructionScript`)