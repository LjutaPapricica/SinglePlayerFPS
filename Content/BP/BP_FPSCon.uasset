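; FPS player controller that forwards movement, look and combat input to the cached BP_FPSPlayer pawn and owns the inventory widget.
; Movement follows camera yaw, or actor rotation while reloading, and reports AI noise from the pawn's calculated loudness.
; Tab toggles inventory and input mode, with an IsInUI macro blocking fire, aim and reload.
; Looping timers drive hold-to-interact, which fills a circular bar, and its cooldown.
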(event `self.ReceiveBeginPlay`
  ;[1 1 1] ゲーム開始時の処理
  (`|ExecutionSequence`
    (:`then_0`
      (bind _asbp_fpsplayer (cast `/Game/BP/BP_FPSPlayer` (`self.K2_GetPawn`)))
      (set `self.PlayerRefe` _asbp_fpsplayer))
    (:`then_1`
      (bind _returnvalue (`|CreateWidget` "/Game/BP/UI/DnDUI/UI_BaseInventory.UI_BaseInventory_C"))
      (bind _output_get (set `self.UI_Inventory` _returnvalue))
      (`/Game/BP/UI/DnDUI/UI_BaseInventory.SlotAdding` _output_get))
    (:`then_2`
      (set `self.GI` (cast `/Game/BP/BP_MyGameInstance` (`GameplayStatics.GetGameInstance`) :!pure true)))))

(event `InputAxis|MoveForward/Backward`
  (params (AxisValue :type "Float (single-precision)"))
  (bind _returnvalue (`self.K2_GetPawn`))
  (bind _playerrefe (`self.PlayerRefe`))
  (bind (_returnvalue_roll _returnvalue_pitch _returnvalue_yaw) (`KismetMathLibrary.BreakRotator` (`self.K2_GetActorRotation` (`GameplayStatics.GetPlayerCameraManager` 0))))
  ;[1 0 0] 動きに関するグラフ
  (`/Game/BP/BP_FPSPlayer.MovePlayer` (`self.PlayerRefe`) (`KismetMathLibrary.GetForwardVector` (`KismetMathLibrary.SelectRotator` (`self.K2_GetActorRotation` _playerrefe) (`KismetMathLibrary.MakeRotator` 0.0 0.0 _returnvalue_yaw) (`/Game/BP/BP_FPSPlayer.isReloading` _playerrefe))) AxisValue)
  (`AISense_Hearing.ReportNoiseEvent` (`self.K2_GetActorLocation` _returnvalue) (`/Game/BP/BP_FPSPlayer.CalculateLoudness` (`self.PlayerRefe`)) _returnvalue :!label _label))

(event `InputAxis|MoveRight/Left`
  (params (AxisValue :type "Float (single-precision)"))
  (bind _playerrefe (`self.PlayerRefe`))
  (bind (_returnvalue_roll _returnvalue_pitch _returnvalue_yaw) (`KismetMathLibrary.BreakRotator` (`self.K2_GetActorRotation` (`GameplayStatics.GetPlayerCameraManager` 0))))
  ;[1 0 0] 動きに関するグラフ
  (`/Game/BP/BP_FPSPlayer.MovePlayer` (`self.PlayerRefe`) (`KismetMathLibrary.GetRightVector` (`KismetMathLibrary.SelectRotator` (`self.K2_GetActorRotation` _playerrefe) (`KismetMathLibrary.MakeRotator` 0.0 0.0 _returnvalue_yaw) (`/Game/BP/BP_FPSPlayer.isReloading` _playerrefe))) AxisValue)
  (goto _label))

(event `InputAxis|LookUp/Down`
  (params (AxisValue :type "Float (single-precision)"))
  ;[1 0 0] 動きに関するグラフ
  (`Pawn.AddControllerPitchInput` (`self.PlayerRefe`) AxisValue))

(event `InputAxis|LookRight/Left`
  (params (AxisValue :type "Float (single-precision)"))
  ;[1 0 0] 動きに関するグラフ
  (`Pawn.AddControllerYawInput` (`self.PlayerRefe`) AxisValue))

(event `InputAction|Run`
  (params (Key :type "Key Structure"))
  ;[1 0 0] 動きに関するグラフ
  (:`Pressed`
    (bind (_direction _alpha) (`Timeline|Run` :!label _label_2)
      (:`Update`
        (`/Game/BP/BP_FPSPlayer.Run` (`self.PlayerRefe`) _alpha))))
  (:`Released`
    (goto _label_2 :!via `Reverse`)))

(event `InputAction|Jump`
  (params (Key :type "Key Structure"))
  ;[1 0 0] 動きに関するグラフ
  (:`Pressed`
    (`Character.Jump` (`self.PlayerRefe`))))

(event `InputAction|Crouch`
  (params (Key :type "Key Structure"))
  (bind _playerrefe (`self.PlayerRefe`))
  ;[1 0 0] 動きに関するグラフ
  (:`Pressed`
    (`/Engine/EditorBlueprintResources/StandardMacros.FlipFlop`
      (:`A`
        (`Character.Crouch` _playerrefe))
      (:`B`
        (`Character.UnCrouch` _playerrefe)))))

(event `InputAction|Aim`
  (params (Key :type "Key Structure"))
  (bind _playerrefe (`self.PlayerRefe`))
  ;[0 0.1405 1] アクションに関するグラフ
  (:`Pressed`
    (`self.IsInUI?`
      (:`false`
        (`/Game/BP/BP_FPSPlayer.StartAim` _playerrefe)
        (set `/Game/BP/BP_FPSPlayer.isAiming` true _playerrefe))))
  (:`Released`
    (`/Game/BP/BP_FPSPlayer.EndAim` _playerrefe)
    (set `/Game/BP/BP_FPSPlayer.isAiming` false _playerrefe)))

(event `InputAction|Fire`
  (params (Key :type "Key Structure"))
  (bind _playerrefe (`self.PlayerRefe`))
  (bind _firehandle (`/Game/BP/BP_FPSPlayer.FireHandle` _playerrefe))
  ;[0 0.1405 1] アクションに関するグラフ
  (:`Pressed`
    (`self.IsInUI?`
      (:`false`
        (`/Game/BP/BP_FPSPlayer.Fire` _playerrefe))))
  (:`Released`
    (if (`KismetSystemLibrary.K2_IsValidTimerHandle` _firehandle)
      (`KismetSystemLibrary.K2_PauseTimerHandle` _firehandle))))

(event `InputAction|Reload`
  (params (Key :type "Key Structure"))
  ;[0 0.1405 1] アクションに関するグラフ
  (:`Pressed`
    (`self.IsInUI?`
      (:`false`
        (`/Game/BP/BP_FPSPlayer.Reload` (`self.PlayerRefe`))))))

(event `InputAction|Interact`
  (params (Key :type "Key Structure"))
  ;[0 0.1405 1] アクションに関するグラフ
  (:`Pressed`
    (if (`self.CanInteract`)
      (`/Game/BP/BP_FPSPlayer.Interact` (`self.PlayerRefe`))
      (bind _returnvalue (`KismetSystemLibrary.K2_SetTimerDelegate` (`|CreateDelegate` :!event `Pressing E Key`) 0.01 true))
      (set `self.InteractHandle` _returnvalue)))
  (:`Released`
    (`self.Released E Key`)))

(event `InteractCoolTime`
  (bind _output_get (set `self.CoolTime` (- (`self.CoolTime`) 0.1)))
  (if (<= _output_get 0.0)
    (`KismetSystemLibrary.K2_PauseTimerHandle` (`self.InteractTimeHandle`))
    (set `self.CoolTime` 2.0)
    (set `self.CanInteract` true)))

(event `Key|Tab`
  (params (Key :type "Key Structure"))
  (bind _ui_inventory (`self.UI_Inventory`))
  (:`Pressed`
    (`/Engine/EditorBlueprintResources/StandardMacros.FlipFlop`
      (:`A`
        (`self.Focus / UnFocusToUI` true :!label _label_3)
        (`UserWidget.AddToViewport` _ui_inventory 0))
      (:`B`
        (`self.Focus / UnFocusToUI` false :!label _label_4)
        (`Widget.RemoveFromParent` _ui_inventory)))))

(event `OpenInventory`
  (goto _label_3))

(event `CloseInventory`
  (goto _label_4))

(event `Key|RightMouseButton`
  (params (Key :type "Key Structure")))

(fn `Focus / UnFocusToUI`
  (params (`ToUI?` :type Boolean))
  (if `ToUI?`
    (`WidgetBlueprintLibrary.SetInputMode_UIOnlyEx` self null)
    (set `self.bShowMouseCursor` true)
    (set `self.isInInventory` true)
    (else
      (`WidgetBlueprintLibrary.SetInputMode_GameOnly` self)
      (bind _output_get (set `self.bShowMouseCursor` false))
      (set `self.isInInventory` _output_get))))

(fn `Pressing E Key`
  (bind _output_get (set `self.ButtonDownTime` (+ (`self.ButtonDownTime`) 0.01)))
  (bind _timeelapsed (`/Game/BP/UI/UI_InteractBar.FillingCircularBar` (`/Game/BP/BP_FPSPlayer.UI_CircularBar` (`self.PlayerRefe`)) _output_get))
  (if _timeelapsed
    (`/Game/BP/BP_FPSPlayer.InteractToItem` (`self.PlayerRefe`))
    (set `self.CanInteract` false)
    (bind _returnvalue (`KismetSystemLibrary.K2_SetTimerDelegate` (`|CreateDelegate` :!event `InteractCoolTime`) 0.1 true))
    (set `self.InteractTimeHandle` _returnvalue)
    (`self.Released E Key`)))

(fn `Released E Key`
  (set `self.ButtonDownTime` 0.0)
  (`/Game/BP/UI/UI_InteractBar.FillingCircularBar` (`/Game/BP/BP_FPSPlayer.UI_CircularBar` (`self.PlayerRefe`)) 0.0)
  (`KismetSystemLibrary.K2_PauseTimerHandle` (`self.InteractHandle`))
  (`/Game/BP/BP_FPSPlayer.CancelInteract` (`self.PlayerRefe`)))

(fn `UserConstructionScript`)