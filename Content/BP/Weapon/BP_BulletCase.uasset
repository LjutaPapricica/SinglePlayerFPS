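; BP_BulletCase is an ejected bullet casing that flies off as a physics object when spawned.
; The construction script applies the Case variable as the static mesh on CaseMesh.
; On BeginPlay it enables physics simulation, then applies a randomized up-and-right impulse.
; The impulse direction comes from player 0's camera rotation rather than the casing's own orientation.
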(event `self.ReceiveBeginPlay`
  (bind _returnvalue (`self.K2_GetActorRotation` (`GameplayStatics.GetPlayerCameraManager` 0)))
  (`|ExecutionSequence`
    (:`then_0`
      (`PrimitiveComponent.SetSimulatePhysics` (`self.CaseMesh`) true))
    (:`then_1`
      (`PrimitiveComponent.AddImpulse` (`self.CaseMesh`) (+ (* (`KismetMathLibrary.GetUpVector` _returnvalue) (`KismetMathLibrary.RandomFloatInRange` 0.3 1.0)) (* (`KismetMathLibrary.GetRightVector` _returnvalue) (`KismetMathLibrary.RandomFloatInRange` 0.5 1.0))) "None" false))))

(fn `UserConstructionScript`
  (`StaticMeshComponent.SetStaticMesh` (`self.CaseMesh`) (`self.Case`)))