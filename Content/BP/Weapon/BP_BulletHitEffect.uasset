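; BP_BulletHitEffect is a bullet impact effect actor that randomizes its look for each instance.
; The construction script picks a random mesh from the Meshes array and gives it a random yaw and uniform scale.
; On BeginPlay it scales the particle system randomly and independently on each axis, then calls Spawned.
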(event `self.ReceiveBeginPlay`
  (bind _returnvalue (`KismetMathLibrary.RandomFloatInRange` 0.1 0.5))
  (`SceneComponent.SetRelativeScale3D` (`self.ParticleSystem1`) (`KismetMathLibrary.MakeVector` _returnvalue _returnvalue _returnvalue))
  (`self.Spawned`))

(fn `UserConstructionScript`
  (bind _staticmesh1 (`self.StaticMesh1`))
  (bind _meshes (`self.Meshes`))
  (`StaticMeshComponent.SetStaticMesh` _staticmesh1 (`|GetArrayItem` _meshes (`KismetMathLibrary.RandomIntegerInRange` 0 (`KismetArrayLibrary.Array_LastIndex` _meshes))))
  (`SceneComponent.K2_SetRelativeRotation` _staticmesh1 (`KismetMathLibrary.MakeRotator` 0.0 0.0 (`KismetMathLibrary.RandomFloatInRange` 0.0 360.0)) false false)
  (`SceneComponent.SetRelativeScale3D` _staticmesh1 (* (`KismetMathLibrary.MakeVector` 1.0 1.0 1.0) (`KismetMathLibrary.RandomFloatInRange` 1.1 1.7))))