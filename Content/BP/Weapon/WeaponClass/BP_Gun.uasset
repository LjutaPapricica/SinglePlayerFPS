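; Gun weapon Blueprint that attaches to a character's mesh and handles aiming, firing and reload animation.
; BeginPlay spawns an iron-sight camera on SightSocket for view-target blending when aiming.
; Fire plays montage and blowback, spawns casing and muzzle/trail effects, then multi-traces with spread for penetration, sending BPI_Destruction damage and spawning Ground impacts.
; Weapon state drives socket names and montage choice; magazine visibility swaps for hand-held reloads.
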(event `self.ReceiveBeginPlay`
  ;[1 1 1] begin play
  (`|ExecutionSequence`
    (:`then_0`
      (bind _returnvalue (`|SpawnActorFromClass` "/Game/BP/Weapon/WeaponClass/BP_IronSightCamera.BP_IronSightCamera_C" (`KismetMathLibrary.MakeTransform` (0.0 0.0 0.0) (`KismetMathLibrary.Conv_VectorToRotator` (`KismetMathLibrary.GreaterGreater_VectorRotator` (1.0 0.0 0.0) (`SceneComponent.K2_GetComponentRotation` (`self.Arrow`))))) "AlwaysSpawn" "OverrideRootScale" null 70.0 null))
      (bind _output_get (set `self.IronSightCamera` _returnvalue))
      (`self.K2_AttachToComponent` _output_get (`self.GunMesh`) "SightSocket" "SnapToTarget" "KeepWorld" "SnapToTarget" true))))

(event `Fire`
  (bind _gunmesh (`self.GunMesh`))
  (bind _gunmesh_2 (`self.GunMesh`))
  (bind _gunmesh_3 (`self.GunMesh`))
  (bind (_s_weaponstate_canselectfiringtype _s_weaponstate_pistol_ _s_weaponstate_clipsize _s_weaponstate_numofcanpenetrate _s_weaponstate_firerate _s_weaponstate_maxbulletspread) (break `/Game/BP/Weapon/s_WeaponState` (`self.s_WeaponState`)))
  (bind _spreadcurrent (`self.SpreadCurrent`))
  (bind _impactpoint (`self.ImpactPoint`))
  (bind (_s_weaponstate_canselectfiringtype_2 _s_weaponstate_pistol__2 _s_weaponstate_clipsize_2 _s_weaponstate_numofcanpenetrate_2) (break `/Game/BP/Weapon/s_WeaponState` (`self.s_WeaponState`)))
  (bind (_returnvalue_location _returnvalue_rotation) (`KismetMathLibrary.BreakTransform` (`SceneComponent.GetSocketTransform` _gunmesh "MuzzleFlashSocket" "RTS_ParentBoneSpace")))
  (bind (_returnvalue_location_2 _returnvalue_rotation_2) (`KismetMathLibrary.BreakTransform` (`SceneComponent.GetSocketTransform` _gunmesh_2 "MuzzleFlashSocket" "RTS_ParentBoneSpace")))
  (bind _returnvalue (`SceneComponent.GetSocketLocation` (`self.GunMesh`) "MuzzleFlashSocket"))
  (bind _returnvalue_2 (`KismetSystemLibrary.MakeLiteralDouble` _s_weaponstate_maxbulletspread))
  ;[1 1 1] Fire
  (`AnimInstance.Montage_Play` (`self.AnimInstance`) "/Game/AnimStarterPack/FireMontage.FireMontage" 1.0 "MontageLength" 0.0 false)
  (`TimelineComponent.PlayFromStart` (`self.BlowBackAnimation`))
  (`|SpawnActorFromClass` "/Game/BP/Weapon/BP_BulletCase.BP_BulletCase_C" (`KismetMathLibrary.MakeTransform` (`SceneComponent.GetSocketLocation` _gunmesh_3 "ShellEjectSocket") (`SceneComponent.GetSocketRotation` _gunmesh_3 "ShellEjectSocket")) "AdjustIfPossibleButDontSpawnIfColliding" "OverrideRootScale" null (`self.BulletCaseMesh`) null)
  (`GameplayStatics.SpawnEmitterAttached` "/Game/Effects/ParticleSystems/Weapons/AssaultRifle/Muzzle/P_AssaultRifle_MF.P_AssaultRifle_MF" _gunmesh_2 "MuzzleFlashSocket" _returnvalue_location_2 _returnvalue_rotation_2 (0.75 0.75 0.75) "SnapToTarget")
  (bind _returnvalue_3 (`GameplayStatics.SpawnEmitterAttached` "/Game/Effects/ParticleSystems/Weapons/AssaultRifle/Muzzle/P_AssaultRifle_Trail.P_AssaultRifle_Trail" _gunmesh "MuzzleFlashSocket" _returnvalue_location _returnvalue_rotation (3.0 3.0 3.0) "SnapToTarget"))
  (set `self.TrailEffect` _returnvalue_3)
  (bind _outhits (`KismetSystemLibrary.LineTraceMulti` :`Start` _returnvalue :`End` (+ (+ _returnvalue (* (`KismetMathLibrary.GetForwardVector` (`self.K2_GetActorRotation` (`GameplayStatics.GetPlayerCameraManager` 0))) 20000.0)) (`KismetMathLibrary.MakeVector` (* _spreadcurrent (`KismetMathLibrary.RandomFloatInRange` (* -1.0 _returnvalue_2) _returnvalue_2)) (* _spreadcurrent (`KismetMathLibrary.RandomFloatInRange` (* -1.0 _returnvalue_2) _returnvalue_2)) (* _spreadcurrent (`KismetMathLibrary.RandomFloatInRange` (* -1.0 _returnvalue_2) _returnvalue_2)))) :`TraceChannel` "TraceTypeQuery3" :`DrawTime` 2.0))
  (bind (_output_bblockinghit _output_binitialoverlap _output_time _output_distance _output_location _output_impactpoint _output_normal _output_impactnormal _output_physmat _output_hitactor _output_hitcomponent _output_hitbonename _output_hititem _output_faceindex _output_tracestart _output_traceend) (`GameplayStatics.BreakHitResult` (`|GetArrayItem` _outhits)))
  (`ParticleSystemComponent.SetBeamTargetPoint` (`self.TrailEffect`) 0 _output_traceend 0)
  (for _index (range _s_weaponstate_numofcanpenetrate_2)
    (bind (_bblockinghit _binitialoverlap _time _distance _location _impactpoint_2 _normal _impactnormal _physmat _hitactor) (`GameplayStatics.BreakHitResult` (`|GetArrayItem` _outhits _index)))
    (set `self.ImpactPoint` _impactpoint_2)
    (set `self.ImpactNormal` _impactnormal)
    (if (`KismetSystemLibrary.DoesImplementInterface` _hitactor "/Game/BP/Interface/BPI_Destruction.BPI_Destruction_C")
      (message `/Game/BP/Interface/BPI_Destruction.Destroy` _hitactor (`self.AntiMatPower`) (`self.ImpactPoint`)))
    (if _bblockinghit
      (switch `EPhysicalSurface` (`PhysicalMaterial.SurfaceType` _physmat)
        (:`SurfaceType_Default`
          (break))
        (:`SurfaceType1`
          (`|SpawnActorFromClass` "/Game/BP/Weapon/BP_BulletHitEffect.BP_BulletHitEffect_C" (`KismetMathLibrary.MakeTransform` (+ (`self.ImpactPoint`) (`self.ImpactNormal`)) (`KismetMathLibrary.FindLookAtRotation` _impactpoint (+ _impactpoint (* (`self.ImpactNormal`) 90.0)))) "AlwaysSpawn" "OverrideRootScale" null null)
          (break))
        (:`SurfaceType2`
          (break))))))

(event `/Game/BP/Weapon/BPI_Weapon.SendSpreadAmount`
  (params (SpreadCurrent :type "Float (single-precision)"))
  (set `self.SpreadCurrent` SpreadCurrent))

(fn `DecreaseMontageLength`
  (set `self.ReloadMontageLength` (- (`self.ReloadMontageLength`) (`GameplayStatics.GetWorldDeltaSeconds`))))

(fn `EndAim`
  (params (NewViewTarget :type "Actor Object Reference"))
  (`PlayerController.SetViewTargetWithBlend` (`GameplayStatics.GetPlayerController` 0) NewViewTarget 0.2 "VTBlend_Linear" 0.0 false))

(fn `MagAttachToHand`
  (params (ParentMesh :type "SceneComponent Object Reference"))
  (bind (_s_weaponstate_canselectfiringtype _s_weaponstate_pistol_ _s_weaponstate_clipsize _s_weaponstate_numofcanpenetrate _s_weaponstate_firerate _s_weaponstate_maxbulletspread _s_weaponstate_firespreadamount _s_weaponstate_fireingtype _s_weaponstate_weaponname) (break `/Game/BP/Weapon/s_WeaponState` (`self.s_WeaponState`)))
  (bind _attachedmag (`self.AttachedMag`))
  (`SceneComponent.K2_AttachToComponent` _attachedmag ParentMesh (`KismetStringLibrary.Conv_StringToName` (`KismetStringLibrary.Concat_StrStr` (`KismetStringLibrary.Conv_NameToString` _s_weaponstate_weaponname) "MagSocket")) "SnapToTarget" "SnapToTarget" "KeepWorld" true)
  (`SceneComponent.SetVisibility` _attachedmag true false)
  (`SceneComponent.SetVisibility` (`self.RealMag`) false false))

(fn `MagDetachFromHand`
  (bind _attachedmag (`self.AttachedMag`))
  (`SceneComponent.K2_DetachFromComponent` _attachedmag "KeepWorld" "KeepWorld" "KeepWorld" true)
  (`SceneComponent.SetVisibility` _attachedmag false false)
  (`SceneComponent.SetVisibility` (`self.RealMag`) true false))

(fn `Reload`
  (bind (_s_weaponstate_canselectfiringtype _s_weaponstate_pistol_) (break `/Game/BP/Weapon/s_WeaponState` (`self.s_WeaponState`)))
  (bind _returnvalue (`AnimInstance.Montage_Play` (`self.AnimInstance`) (select `bool` _s_weaponstate_pistol_ :`false` "/Game/AnimStarterPack/ReloadMontage.ReloadMontage" :`true` "/Game/AnimStarterPack/SMGReloadMontage.SMGReloadMontage" :!type "AnimMontage Object Reference") 1.0 "MontageLength" 0.0 false))
  (set `self.ReloadMontageLength` _returnvalue))

(fn `SpawnEquip`
  (params (ParentMeshComp :type "SkeletalMeshComponent Object Reference"))
  (bind (_s_weaponstate_canselectfiringtype _s_weaponstate_pistol_ _s_weaponstate_clipsize _s_weaponstate_numofcanpenetrate _s_weaponstate_firerate _s_weaponstate_maxbulletspread _s_weaponstate_firespreadamount _s_weaponstate_fireingtype _s_weaponstate_weaponname) (break `/Game/BP/Weapon/s_WeaponState` (`self.s_WeaponState`)))
  (`SceneComponent.K2_AttachToComponent` (`self.GunMesh`) ParentMeshComp (`KismetStringLibrary.Conv_StringToName` (`KismetStringLibrary.Concat_StrStr` (`KismetStringLibrary.Conv_NameToString` _s_weaponstate_weaponname) "GunSocket")) "SnapToTarget" "SnapToTarget" "KeepWorld" true)
  (bind _asabp_fpsplayer (cast `/Game/BP/ABP_FPSPlayer` (`SkeletalMeshComponent.GetAnimInstance` ParentMeshComp)))
  (set `self.AnimInstance` _asabp_fpsplayer))

(fn `StartAim`
  (`PlayerController.SetViewTargetWithBlend` (`GameplayStatics.GetPlayerController` 0) (`self.IronSightCamera`) 0.125 "VTBlend_Cubic" 2.0 false))

(fn `UserConstructionScript`)