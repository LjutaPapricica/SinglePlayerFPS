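; Base AI controller for shooter enemies that runs the BT_Shooter behavior tree on the BB_Shooter blackboard, starting out of combat mode.
; PawnSensing writes heard noise location and instigator to the blackboard, while seen pawns are only cached in SawActor.
; Helper functions store patrol location actors, clear noise info, set the shooter type key and reset the combat flag, which SetisCombatMode always sets false.
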(event `self.ReceiveBeginPlay`
  (`|ExecutionSequence`
    (:`then_0`
      (`self.RunBehaviorTree` "/Game/BP/ShooterAI/BT/BT_Shooter.BT_Shooter")
      (bind _blackboardcomponent (`self.UseBlackboard` "/Game/BP/ShooterAI/BT/BB_Shooter.BB_Shooter"))
      (set `self.BBComp` _blackboardcomponent))
    (:`then_1`
      (`self.SetisCombatMode`))))

(event `self.PawnSensing.OnHearNoise`
  (params (Instigator :type "Pawn Object Reference") (Location :type "Vector Structure (by ref)") (Volume :type "Float (single-precision)"))
  (bind _output_get (set `self.NoiseLocation` Location))
  (`BlackboardComponent.SetValueAsVector` (`self.BBComp`) "NoiseLocation" _output_get)
  (bind _output_get_2 (set `self.NoiseMadeActor` Instigator))
  (`BlackboardComponent.SetValueAsObject` (`self.BBComp`) "NoiseMadeActor" _output_get_2))

(event `self.PawnSensing.OnSeePawn`
  (params (Pawn :type "Pawn Object Reference"))
  (set `self.SawActor` Pawn))

(fn `ForgetNoiseInfo`
  (returns (`ForgetSuccessfully?` :type Boolean))
  (bind _output_get (set `self.NoiseLocation` (0.0 0.0 0.0)))
  (`BlackboardComponent.SetValueAsVector` (`self.BBComp`) "NoiseLocation" _output_get)
  (bind _output_get_2 (set `self.NoiseMadeActor` null))
  (`BlackboardComponent.SetValueAsObject` (`self.BBComp`) "NoiseMadeActor" _output_get_2)
  (return (not (`KismetSystemLibrary.IsValid` (`self.NoiseMadeActor`)))))

(fn `SetisCombatMode`
  (`BlackboardComponent.SetValueAsBool` (`self.BBComp`) "isCombatMode" false))

(fn `SetPatrolLocationActors`
  (params (PatrolLocationActors :type "Array of TargetPoint Object Reference"))
  (set `self.PatrolLocationActors` PatrolLocationActors))

(fn `SetShooterType`
  (params (EnumValue :type Byte))
  (`BlackboardComponent.SetValueAsEnum` (`self.BBComp`) "e_ShooterType" EnumValue))

(fn `UserConstructionScript`)