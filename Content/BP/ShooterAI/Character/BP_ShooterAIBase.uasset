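; Base character for AI shooters, with body tint, crouch, sprint, hit reactions and death.
; BeginPlay attaches a spawned AK to the spine socket and passes patrol points and shooter type to the AI controller.
; Tick feeds smoothed aim pitch/yaw to the AnimBP, turning the actor at large yaw.
; Damage triggers effects, montage and knockback, while OnRep_HP handles death by stopping AI, ragdolling and breaking hit limb constraints for dismemberment.
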(fn `CanDismemberment`
  (returns (CanDismemberment :type Boolean))
  (switch `name` (`self.HitBoneName`)
    (:`Default`
      (return false))
    (:`upperarm_r`
      _)
    (:`upperarm_l`
      _)
    (:`lowerarm_r`
      _)
    (:`lowerarm_l`
      _)
    (:`hand_r`
      _)
    (:`hand_l`
      _)
    (:`thigh_r`
      _)
    (:`thigh_l`
      _)
    (:`calf_r`
      _)
    (:`calf_l`
      _))
  (return true))

(fn `DeathAnim`
  (bind _mesh (`self.Mesh`))
  (bind _hitbonename (`self.HitBoneName`))
  (`PrimitiveComponent.SetSimulatePhysics` _mesh true)
  (`PrimitiveComponent.AddImpulseAtLocation` _mesh (* (+ (* (`KismetMathLibrary.GetForwardVector` (`self.K2_GetActorRotation` (`GameplayStatics.GetPlayerPawn` 0))) 5000.0) (* (`self.GetActorUpVector`) 5000.0)) (`KismetMathLibrary.VSize` (`self.GetVelocity`))) (`SceneComponent.GetSocketLocation` (`self.Mesh`) _hitbonename) _hitbonename)
  (bind _candismemberment (`self.CanDismemberment`))
  (if _candismemberment
    (`SkeletalMeshComponent.BreakConstraint` (`self.Mesh`) (+ (* (`self.GetActorUpVector`) 333.0) (* (`KismetMathLibrary.GetForwardVector` (`self.K2_GetActorRotation` (`GameplayStatics.GetPlayerPawn` 0))) 1250.0)) (`SceneComponent.GetSocketLocation` (`self.Mesh`) (`self.HitBoneName`)) (`self.HitBoneName`))
    (`GameplayStatics.SpawnSoundAtLocation` "/Game/Sounds/FoleyFlesh/Stereo/Dismemberment_Cue.Dismemberment_Cue" (`self.K2_GetActorLocation`) (struct) 1.0 1.0 0.0 null null)))

(fn `EndCrouch`
  (`self.UnCrouch`)
  (message `/Game/BP/Interface/BPI_Animation.EndCrouch` (`self.AnimInstance`) false))

(fn `EndSprint`
  (message `/Game/BP/Interface/BPI_Animation.EndSprint` (`self.AnimInstance`) false))

(fn `OnRep_HP`
  (if (and (<= (`self.HP`) 0.0) (not (`self.isDead`)))
    (`MovementComponent.StopMovementImmediately` (`self.CharacterMovement`))
    (`PrimitiveComponent.SetCollisionEnabled` (`self.CapsuleComponent`) "NoCollision")
    (`BrainComponent.StopLogic` (`AIController.BrainComponent` (`AIBlueprintHelperLibrary.GetAIController` self)) "")
    (set `self.isDead` true)
    (`self.DeathAnim`)))

(fn `PlayEquipWeaponMontage`
  (returns (MontageDuration :type "Float (double-precision)"))
  (bind _returnvalue (`AnimInstance.Montage_Play` (`self.AnimInstance`) "/Game/AnimStarterPack/EquipWeapon.EquipWeapon" 1.0 "Duration" 0.0 true))
  (return _returnvalue))

(fn `SprintToWalk`
  (returns (ReturnValue :type Boolean))
  (bind _output_get (set `CharacterMovementComponent.MaxWalkSpeed` (`KismetMathLibrary.FInterpTo` (`CharacterMovementComponent.MaxWalkSpeed` (`self.CharacterMovement`)) 450.0 (`GameplayStatics.GetWorldDeltaSeconds`) 4.0) (`self.CharacterMovement`)))
  (if (`KismetMathLibrary.NearlyEqual_FloatFloat` _output_get 450.0 1.0)
    (return true)))

(fn `StartCrouch`
  (`self.Crouch`)
  (message `/Game/BP/Interface/BPI_Animation.StartCrouch` (`self.AnimInstance`) true))

(fn `StartSprint`
  (message `/Game/BP/Interface/BPI_Animation.StartSprint` (`self.AnimInstance`) true))

(fn `UserConstructionScript`
  (bind _returnvalue (`PrimitiveComponent.CreateDynamicMaterialInstance` (`self.Mesh`) 0 null "None"))
  (`MaterialInstanceDynamic.SetVectorParameterValue` _returnvalue "BodyColor" (`self.BodyColor`)))

(fn `WalkToSprint`
  (returns (ReturnValue :type Boolean))
  (bind _output_get (set `CharacterMovementComponent.MaxWalkSpeed` (`KismetMathLibrary.FInterpTo` (`CharacterMovementComponent.MaxWalkSpeed` (`self.CharacterMovement`)) 450.0 (`GameplayStatics.GetWorldDeltaSeconds`) 4.0) (`self.CharacterMovement`)))
  (if (`KismetMathLibrary.NearlyEqual_FloatFloat` _output_get 450.0 1.0)
    (return true)))